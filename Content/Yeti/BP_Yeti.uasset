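; BP_Yeti is an enemy that throws snowballs at the player character when it sees them.
; PawnSensing sightings of BP_ThirdPersonCharacter snap the Yeti's rotation toward the target and, if CanAttack is set, spawn a BP_snowball at SpawnSnowBallLocation.
; Damage is applied directly to the player at throw time, independent of any snowball hit.
; A short delay on CanAttack serves as the attack cooldown.
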(event `self.PawnSensing.OnSeePawn`
  (params (Pawn :type "Pawn Object Reference"))
  (bind _asbp_third_person_character (cast `/Game/Player/BP_ThirdPersonCharacter` Pawn))
  (`self.K2_SetActorRotation` (`KismetMathLibrary.FindRelativeLookAtRotation` (`KismetMathLibrary.Conv_VectorToTransform` (`self.K2_GetActorLocation`)) (`self.K2_GetActorLocation` _asbp_third_person_character)))
  (if (`self.CanAttack?`)
    (`|SpawnActorFromClass` "/Game/Yeti/BP_snowball.BP_snowball_C" (`SceneComponent.K2_GetComponentToWorld` (`self.SpawnSnowBallLocation`)) "Undefined" "MultiplyWithRoot" null null)
    (`GameplayStatics.ApplyDamage` _asbp_third_person_character 1.0)
    (set `self.CanAttack?` false)
    (`KismetSystemLibrary.Delay` 1.0)
    (set `self.CanAttack?` true)))

(fn `UserConstructionScript`)